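; BP_kartka_fake2 is a fake note ("kartka") actor that shows its texture on screen and destroys itself when overlapped.
; On overlap it sends ChangeSpeedMessage to every Speedinterface actor, then creates a WBP_KartkaViewer_Fake2 widget with TeksturaKartki.
; A timer set on end overlap targets Zamknij_kartke, which removes KartkaWidget.
; The new widget is never stored in KartkaWidget here, and the actor is destroyed right after display.
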(event Custom|zamknij_kartke
  ;[0.15 0.15 0.15 0.5] wyswietlanie kartek
  (if (Utilities|IsValid (Variables|Default|Getkartka_widget))
    (Widget|RemovefromParent (Variables|Default|Getkartka_widget))))

(event Collision|EventActorBeginOverlap
  (params (OtherActor :type Actor%20Object%20Reference))
  (Actor|GetAllActorswithInterface "/Game/ThirdPerson/Blueprints/speedinterface.speedinterface_C")
  (Utilities|FlowControl|Sequence
    (:then_0
      (for _array_element 0
        (Class|Speedinterface|ChangeSpeed(Message) _array_element)))
    (:then_1
      (bind _returnvalue (UserInterface|CreateWidget "/Game/Hubert_vel_hitruss/WBP_KartkaViewer_Fake2.WBP_KartkaViewer_Fake2_C"))
      (bind _aswbp_kartka_viewer_fake_2 (Utilities|Casting|CastToWBP_KartkaViewer_Fake2 _returnvalue))
      (CallFunction|ZamknijKartke)
      (Appearance|SetBrushfromTexture (Variables|/Game/Hubert_vel_hitruss/WBP_KartkaViewer_Fake2.WBP_KartkaViewer_Fake2_C|GetKartka_image _aswbp_kartka_viewer_fake_2) (Variables|Default|Gettekstura_kartki) false)
      (UserInterface|Viewport|AddtoViewport _returnvalue 0)
      (Actor|DestroyActor) ; destroy actor opcjonalne, w przypadku jednorazoego pjawiania sie kartek
    )))

(event Collision|EventActorEndOverlap
  (params (OtherActor :type Actor%20Object%20Reference))
  ;[0.15 0.15 0.15 0.5] wyswietlanie kartek
  (Utilities|Time|SetTimerbyEvent (delegate Custom|zamknij_kartke) 3.0) ; długosc wyswietlania na ekranie
)

(fn ConstructionScript)