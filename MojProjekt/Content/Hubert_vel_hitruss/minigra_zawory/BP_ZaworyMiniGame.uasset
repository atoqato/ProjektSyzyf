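; Valve-turning minigame actor with three clickable valves, each click rotating its valve a step further.
; Overlapping InteractZone while unsolved freezes the character, enables mouse clicks and blends the camera to the actor.
; Escape, debug R or Zakonczenie restores camera and controls.
; Tick flags completion and calls Zakonczenie without checking valve progress, so the logic appears unfinished; the code-panel widget is created but never shown.
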(event OnComponentBeginOverlap(InteractZone)
  (params (OverlappedComponent :type Primitive%20Component%20Object%20Reference) (OtherActor :type Actor%20Object%20Reference) (OtherComp :type Primitive%20Component%20Object%20Reference) (OtherBodyIndex :type Integer) (bFromSweep :type Boolean) (SweepResult :type Hit%20Result%20Structure%20%28by%20ref%29))
  (bind _returnvalue (Game|GetPlayerController 0))
  (bind _returnvalue_2 (Game|GetPlayerController 0))
  ;[0.15 0.15 0.15 0.5] lockowanie kamery gracza i cinematic przejscie
  (if (not (Variables|Default|GetisZakrecone))
    (bind _asbp_third_person_character (Utilities|Casting|CastToBP_ThirdPersonCharacter OtherActor))
    (Variables|/Script/Engine.PlayerController|SetbEnableClickEvents _returnvalue true)
    (Variables|/Script/Engine.PlayerController|SetbShowMouseCursor _returnvalue true)
    (Pawn|Components|CharacterMovement|SetMovementMode (Variables|/Script/Engine.Character|GetCharacterMovement _asbp_third_person_character) "MOVE_None" 0)
    (Input|SetInputModeGameandUI (Game|GetPlayerController 0) 0 "DoNotLock" true false)
    (Input|SetIgnoreLookInput _returnvalue_2 true)
    (Game|Player|SetViewTargetwithBlend _returnvalue_2 self 1.2 "VTBlend_Cubic" 0.0 true)
    (Variables|Default|SetcwelObrotowy true)))

(event OnComponentEndOverlap(InteractZone)
  (params (OverlappedComponent :type Primitive%20Component%20Object%20Reference) (OtherActor :type Actor%20Object%20Reference) (OtherComp :type Primitive%20Component%20Object%20Reference) (OtherBodyIndex :type Integer))
  ;[0.15 0.15 0.15 0.5] Wyjscie z kolizji z obiektem
)

(event OnClicked(zawor3)
  (params (TouchedComponent :type Primitive%20Component%20Object%20Reference) (ButtonPressed :type Key%20Structure :default "None"))
  (Development|PrintString "3 klik")
  (Variables|Default|SetPostep3 (+ (Variables|Default|GetPostep3) 0.1))
  (Transformation|SetRelativeRotation (Variables|Default|Getzawor3) (Math|Rotator|MakeRotator 0.0 (* (Variables|Default|GetPostep3) 9e+01) 0.0) false false))

(event OnClicked(zawor2)
  (params (TouchedComponent :type Primitive%20Component%20Object%20Reference) (ButtonPressed :type Key%20Structure :default "None"))
  (Development|PrintString "2 klik")
  (Variables|Default|SetPostep2 (+ (Variables|Default|GetPostep2) 0.1))
  (Transformation|SetRelativeRotation (Variables|Default|Getzawor2) (Math|Rotator|MakeRotator 0.0 (* (Variables|Default|GetPostep2) -9e+01) 0.0) false false))

(event OnClicked(zawor1)
  (params (TouchedComponent :type Primitive%20Component%20Object%20Reference) (ButtonPressed :type Key%20Structure :default "None"))
  (Development|PrintString "1 klik")
  (Variables|Default|SetPostep1 (+ (Variables|Default|GetPostep1) 0.1))
  (Transformation|SetRelativeRotation (Variables|Default|Getzawor1) (Math|Rotator|MakeRotator 0.0 (* (Variables|Default|GetPostep1) 9e+01) 0.0) false false))

(event Custom|zakonczenie
  (bind _returnvalue (Game|GetPlayerController 0))
  ;[0.15 0.15 0.15 0.5] Zamykanie widgetu po wcisnieciu R (dev) lub ESC
  (if true
    (Game|Player|SetViewTargetwithBlend (Game|GetPlayerController 0) (Game|GetPlayerCharacter 0) 1.2 "VTBlend_Cubic" 0.0 true)
    (Input|SetIgnoreLookInput _returnvalue false)
    (Input|SetInputModeGameOnly _returnvalue false)
    (Variables|/Script/Engine.PlayerController|SetbShowMouseCursor _returnvalue false)
    (bind _asbp_third_person_character (Utilities|Casting|CastToBP_ThirdPersonCharacter (Game|GetPlayerCharacter 0)))
    (Pawn|Components|CharacterMovement|SetMovementMode (Variables|/Script/Engine.Character|GetCharacterMovement _asbp_third_person_character) "MOVE_Walking" 0)))

(event EventBeginPlay
  ;[0.15 0.15 0.15 0.5] Tworzenie widgetu przy starcie
  (bind _returnvalue (UserInterface|CreateWidget "/Game/Igor/WBP_CodePanel.WBP_CodePanel_C"))
  (Variables|Default|SetCodePanelWidget _returnvalue))

(event EventTick
  (params (DeltaSeconds :type Float%20%28single-precision%29))
  (if (and (!= (Variables|Default|GetisZakrecone) false) (Variables|Default|GetcwelObrotowy))
    (Variables|Default|SetPostep1 (- (Variables|Default|GetPostep1) -0.05))
    (Transformation|SetRelativeRotation (Variables|Default|Getzawor1) (Math|Rotator|MakeRotator 0.0 -1e+01 0.0) false false)
    (else
      (Variables|Default|SetisZakrecone true)
      (CallFunction|Zakonczenie))))

(event Input|KeyboardEvents|DebugKeyR
  (params (Key :type Key%20Structure :default "None") (ActionValue :type Input%20Action%20Value%20Structure))
  (bind _returnvalue (Game|GetPlayerController 0))
  ;[0.15 0.15 0.15 0.5] Zamykanie widgetu po wcisnieciu R (dev) lub ESC
  (:Pressed
    (if true
      (Game|Player|SetViewTargetwithBlend (Game|GetPlayerController 0) (Game|GetPlayerCharacter 0) 1.2 "VTBlend_Cubic" 0.0 true)
      (Input|SetIgnoreLookInput _returnvalue false)
      (Input|SetInputModeGameOnly _returnvalue false)
      (Variables|/Script/Engine.PlayerController|SetbShowMouseCursor _returnvalue false)
      (bind _asbp_third_person_character (Utilities|Casting|CastToBP_ThirdPersonCharacter (Game|GetPlayerCharacter 0)))
      (Pawn|Components|CharacterMovement|SetMovementMode (Variables|/Script/Engine.Character|GetCharacterMovement _asbp_third_person_character) "MOVE_Walking" 0))))

(event Input|KeyboardEvents|Escape
  (params (Key :type Key%20Structure :default "None"))
  (bind _returnvalue (Game|GetPlayerController 0))
  ;[0.15 0.15 0.15 0.5] Zamykanie widgetu po wcisnieciu R (dev) lub ESC
  (:Pressed
    (if true
      (Game|Player|SetViewTargetwithBlend (Game|GetPlayerController 0) (Game|GetPlayerCharacter 0) 1.2 "VTBlend_Cubic" 0.0 true)
      (Input|SetIgnoreLookInput _returnvalue false)
      (Input|SetInputModeGameOnly _returnvalue false)
      (Variables|/Script/Engine.PlayerController|SetbShowMouseCursor _returnvalue false)
      (bind _asbp_third_person_character (Utilities|Casting|CastToBP_ThirdPersonCharacter (Game|GetPlayerCharacter 0)))
      (Pawn|Components|CharacterMovement|SetMovementMode (Variables|/Script/Engine.Character|GetCharacterMovement _asbp_third_person_character) "MOVE_Walking" 0))))

(fn ConstructionScript)