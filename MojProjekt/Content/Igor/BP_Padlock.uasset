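; BP_Padlock is a world padlock that shows a code-entry panel when the player character enters its interact zone.
; It creates WBP_CodePanel at BeginPlay as its owner; on overlap, if still locked, it displays the panel, freezes movement and look, and shows the cursor.
; Escape or debug R closes the panel and restores walking, while leaving the zone restores look input.
; The OnPadlockUnlocked event plays an unlock sound and destroys the actor.
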(event OnComponentBeginOverlap(InteractZone)
  (params (OverlappedComponent :type Primitive%20Component%20Object%20Reference) (OtherActor :type Actor%20Object%20Reference) (OtherComp :type Primitive%20Component%20Object%20Reference) (OtherBodyIndex :type Integer) (bFromSweep :type Boolean) (SweepResult :type Hit%20Result%20Structure%20%28by%20ref%29))
  ;[0.15 0.15 0.15 0.5] Otwieranie widgetu przy wejściu w strefę kłódki
  (if (not (Variables|Default|GetIsOpened))
    (if (not (Variables|Default|GetbUnlocked))
      (Development|PrintString (Utilities|String|ToString(Boolean) (Variables|Default|GetbUnlocked)))
      (Variables|Default|SetIsOpened true)
      (Input|SetIgnoreLookInput (Game|GetPlayerController 0) true)
      (bind _asbp_third_person_character (Utilities|Casting|CastToBP_ThirdPersonCharacter OtherActor))
      (UserInterface|Viewport|AddtoViewport (Variables|Default|GetCodePanelWidget) 0)
      (Input|SetInputModeGameandUI (Game|GetPlayerController 0) (Variables|Default|GetCodePanelWidget) "DoNotLock" true false)
      (Variables|/Script/Engine.PlayerController|SetbShowMouseCursor (Game|GetPlayerController 0) true)
      (Pawn|Components|CharacterMovement|SetMovementMode (Variables|/Script/Engine.Character|GetCharacterMovement _asbp_third_person_character) "MOVE_None" 0))))

(event OnComponentEndOverlap(InteractZone)
  (params (OverlappedComponent :type Primitive%20Component%20Object%20Reference) (OtherActor :type Actor%20Object%20Reference) (OtherComp :type Primitive%20Component%20Object%20Reference) (OtherBodyIndex :type Integer))
  ;[0.15 0.15 0.15 0.5] Wyjscie z kolizji z kłódką
  (Variables|Default|SetIsOpened false)
  (Input|SetIgnoreLookInput (Game|GetPlayerController 0) false))

(event Custom|Destroy
  ;[0.15 0.15 0.15 0.5] Tworzenie widgetu przy starcie
  (Audio|PlaySoundatLocation "/Game/Audio/odblokowanieklodki.odblokowanieklodki" (Variables|/Script/Engine.SceneComponent|GetRelativeLocation (Variables|Default|GetDefaultSceneRoot)) "0, 0, 0" 1.0 1.0 0.0 0 0 0 0)
  (Actor|DestroyActor))

(event EventBeginPlay
  ;[0.15 0.15 0.15 0.5] Tworzenie widgetu przy starcie
  (bind _returnvalue (UserInterface|CreateWidget "/Game/Igor/WBP_CodePanel.WBP_CodePanel_C"))
  (Variables|Default|SetCodePanelWidget _returnvalue)
  (Variables|/Game/Igor/WBP_CodePanel.WBP_CodePanel_C|SetOwningPadlock _returnvalue self)
  (EventDispatchers|BindEventtoOnPadlockUnlocked (delegate Custom|Destroy)))

(event Input|KeyboardEvents|DebugKeyR
  (params (Key :type Key%20Structure :default "None") (ActionValue :type Input%20Action%20Value%20Structure))
  ;[0.15 0.15 0.15 0.5] Zamykanie widgetu po wcisnieciu R (dev) lub ESC
  (:Pressed
    (if (Variables|Default|GetIsOpened)
      (bind _foundwidgets (Widget|GetAllWidgetsOfClass "/Game/Igor/WBP_CodePanel.WBP_CodePanel_C" true))
      (Widget|RemovefromParent (Utilities|Array|Get(acopy) _foundwidgets))
      (Input|SetInputModeGameOnly (Game|GetPlayerController 0) false)
      (Variables|/Script/Engine.PlayerController|SetbShowMouseCursor (Game|GetPlayerController 0) false)
      (bind _asbp_third_person_character (Utilities|Casting|CastToBP_ThirdPersonCharacter (Game|GetPlayerCharacter 0)))
      (Pawn|Components|CharacterMovement|SetMovementMode (Variables|/Script/Engine.Character|GetCharacterMovement _asbp_third_person_character) "MOVE_Walking" 0))))

(event Input|KeyboardEvents|Escape
  (params (Key :type Key%20Structure :default "None"))
  ;[0.15 0.15 0.15 0.5] Zamykanie widgetu po wcisnieciu R (dev) lub ESC
  (:Pressed
    (if (Variables|Default|GetIsOpened)
      (bind _foundwidgets (Widget|GetAllWidgetsOfClass "/Game/Igor/WBP_CodePanel.WBP_CodePanel_C" true))
      (Widget|RemovefromParent (Utilities|Array|Get(acopy) _foundwidgets))
      (Input|SetInputModeGameOnly (Game|GetPlayerController 0) false)
      (Variables|/Script/Engine.PlayerController|SetbShowMouseCursor (Game|GetPlayerController 0) false)
      (bind _asbp_third_person_character (Utilities|Casting|CastToBP_ThirdPersonCharacter (Game|GetPlayerCharacter 0)))
      (Pawn|Components|CharacterMovement|SetMovementMode (Variables|/Script/Engine.Character|GetCharacterMovement _asbp_third_person_character) "MOVE_Walking" 0))))

(fn ConstructionScript)